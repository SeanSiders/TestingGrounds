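; Behavior tree task that makes an AI-controlled BP_Character aim and shoot at its blackboard Target.
; On execute it turns on the character's Aiming and Shooting flags and sets the controller's focus to the Target actor.
; It never finishes execution on its own, so it runs until aborted.
; On abort it clears both flags and the focus, then finishes the abort.
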(event EventReceiveExecuteAI
  (params (OwnerController :type AI%20Controller%20Object%20Reference) (ControlledPawn :type Pawn%20Object%20Reference))
  (bind _asbp_character (Utilities|Casting|CastToBP_Character ControlledPawn))
  (bind _output_get (Variables|/Game/Dynamic/Character/Behaviour/BP_Character.BP_Character_C|SetAiming _asbp_character true))
  (Variables|/Game/Dynamic/Character/Behaviour/BP_Character.BP_Character_C|SetShooting _asbp_character _output_get)
  (AI|SetFocus OwnerController (AI|BehaviorTree|GetBlackboardValueasActor (Variables|Default|GetTarget))))

(event EventReceiveAbortAI
  (params (OwnerController :type AI%20Controller%20Object%20Reference) (ControlledPawn :type Pawn%20Object%20Reference))
  (bind _asbp_character (Utilities|Casting|CastToBP_Character ControlledPawn))
  (bind _output_get (Variables|/Game/Dynamic/Character/Behaviour/BP_Character.BP_Character_C|SetAiming _asbp_character false))
  (Variables|/Game/Dynamic/Character/Behaviour/BP_Character.BP_Character_C|SetShooting _asbp_character _output_get)
  (AI|ClearFocus OwnerController)
  (Class|BTTaskBlueprintBase|FinishAbort))