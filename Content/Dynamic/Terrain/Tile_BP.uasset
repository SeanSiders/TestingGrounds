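; Tile_BP is a terrain tile for infinite terrain, with a barrier, trigger volumes and an arrow transform that serves as an attach location.
; The barrier starts locked (red, collidable) and unlocks (green, no collision) while the player character overlaps LockingVolume.
; Leaving that volume relocks it and asks InfiniteTerrainGameMode_BP to spawn tiles.
; Player overlap with LevelDestroyVolume destroys the tile.
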(event OnComponentEndOverlap(LockingVolume)
  (params (OverlappedComponent :type Primitive%20Component%20Object%20Reference) (OtherActor :type Actor%20Object%20Reference) (OtherComp :type Primitive%20Component%20Object%20Reference) (OtherBodyIndex :type Integer))
  (Utilities|IsPlayerCharacter OtherActor)
  (CallFunction|LockLevel)
  (bind _asinfinite_terrain_game_mode_bp (Utilities|Casting|CastToInfiniteTerrainGameMode_BP (Game|GetGameMode)))
  (Default|SpawnTiles _asinfinite_terrain_game_mode_bp))

(event OnComponentBeginOverlap(LockingVolume)
  (params (OverlappedComponent :type Primitive%20Component%20Object%20Reference) (OtherActor :type Actor%20Object%20Reference) (OtherComp :type Primitive%20Component%20Object%20Reference) (OtherBodyIndex :type Integer) (bFromSweep :type Boolean) (SweepResult :type Hit%20Result%20Structure%20%28by%20ref%29))
  (Utilities|IsPlayerCharacter OtherActor)
  (CallFunction|UnlockLevel))

(event OnComponentBeginOverlap(LevelDestroyVolume)
  (params (OverlappedComponent :type Primitive%20Component%20Object%20Reference) (OtherActor :type Actor%20Object%20Reference) (OtherComp :type Primitive%20Component%20Object%20Reference) (OtherBodyIndex :type Integer) (bFromSweep :type Boolean) (SweepResult :type Hit%20Result%20Structure%20%28by%20ref%29))
  (Utilities|IsPlayerCharacter OtherActor)
  (Actor|DestroyActor))

(event EventBeginPlay
  (CallFunction|LockLevel))

(fn ConstructionScript)

(fn GetAttachLocation
  (return (Transformation|GetWorldTransform (Variables|Default|GetArrow))))

(fn UnlockLevel
  (Collision|SetCollisionEnabled (Variables|Default|GetBarrier) "NoCollision")
  (Rendering|Material|SetMaterial (Variables|Default|GetBarrier) 0 "/Game/Dynamic/Terrain/Barrier_Green.Barrier_Green"))

(fn LockLevel
  (Collision|SetCollisionEnabled (Variables|Default|GetBarrier) "QueryAndPhysics")
  (Rendering|Material|SetMaterial (Variables|Default|GetBarrier) 0 "/Game/Dynamic/Terrain/Barrier_Red.Barrier_Red"))